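; Enemy Blueprint that melee-attacks the player, takes bullet damage and shows a health bar bound to itself.
; Mesh and capsule hits from damaging objects subtract health scaled by the player's GunLevel and destroy the bullet; capsule hits on kill boxes destroy the enemy.
; Tick sets AutoDestroyWhenFinished from the health component's Alive state, then damages the player when overlapping the attack box and the cooldown has elapsed.
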(event `self.ReceiveBeginPlay`
  (`self.Init Health Bar`))

(event `self.Mesh.OnComponentHit`
  (params (HitComponent :type "PrimitiveComponent Object Reference") (OtherActor :type "Actor Object Reference") (OtherComp :type "PrimitiveComponent Object Reference") (NormalImpulse :type "Vector Structure") (Hit :type "HitResult Structure (by ref)"))
  (switch `ECollisionChannel` (`PrimitiveComponent.GetCollisionObjectType` OtherComp)
    (:`ECC_GameTraceChannel2`
      (bind _asplayer_bp (cast `/Game/UnrealGameBP/Player/PlayerBP` (`GameplayStatics.GetPlayerCharacter` 0)))
      (`/Game/UnrealGameBP/Components/PawnHealthComponent.Hit` (`self.PawnHealthComponent`) (* (`/Game/UnrealGameBP/Player/PlayerBP.Gun Level` _asplayer_bp) 5.0))
      (`self.K2_DestroyActor` OtherActor) ; Destroy bullet
    )))

(event `self.CapsuleComponent.OnComponentHit`
  (params (HitComponent :type "PrimitiveComponent Object Reference") (OtherActor :type "Actor Object Reference") (OtherComp :type "PrimitiveComponent Object Reference") (NormalImpulse :type "Vector Structure") (Hit :type "HitResult Structure (by ref)"))
  (switch `ECollisionChannel` (`PrimitiveComponent.GetCollisionObjectType` OtherComp)
    (:`ECC_GameTraceChannel2`
      (bind _asplayer_bp (cast `/Game/UnrealGameBP/Player/PlayerBP` (`GameplayStatics.GetPlayerCharacter` 0)))
      (`/Game/UnrealGameBP/Components/PawnHealthComponent.Hit` (`self.PawnHealthComponent`) (* (`/Game/UnrealGameBP/Player/PlayerBP.Gun Level` _asplayer_bp) 5.0))
      (`self.K2_DestroyActor` OtherActor) ; Destroy bullet
    )
    (:`ECC_GameTraceChannel5`
      (`self.K2_DestroyActor`))))

(event `self.ReceiveTick`
  (params (DeltaSeconds :type "Float (single-precision)"))
  (`|ExecutionSequence`
    (:`then_0`
      (`self.CheckLiving`))
    (:`then_1`
      (bind _canattack (`self.CheckAttackPossible` DeltaSeconds))
      (if _canattack
        (`self.Attack`)))))

(fn `Attack`
  (bind _asplayer_bp (cast `/Game/UnrealGameBP/Player/PlayerBP` (`GameplayStatics.GetPlayerCharacter` 0)))
  (`/Game/UnrealGameBP/Player/PlayerBP.Take Damage` _asplayer_bp (`self.AttackPower`))
  (set `self.Time Since Attack` 0.0))

(fn `CheckAttackPossible`
  (params (`Delta S` :type "Float (double-precision)"))
  (returns (CanAttack :type Boolean))
  (set `self.Time Since Attack` (+ `Delta S` (`self.Time Since Attack`)))
  (if (`PrimitiveComponent.IsOverlappingActor` (`self.Box`) (`GameplayStatics.GetPlayerCharacter` 0))
    (`/Engine/EditorBlueprintResources/StandardMacros.CompareFloat` (`self.Time Since Attack`) (`self.Attack Cooldown`)
      (:`>`
        (set `self.CanAttack` true :!label _label))
      (:`==`
        (goto _label))
      (:`<`
        (set `self.CanAttack` false)))
    (return (`self.CanAttack`))))

(fn `CheckLiving`
  (set `self.bAutoDestroyWhenFinished` (not (`/Game/UnrealGameBP/Components/PawnHealthComponent.Alive` (`self.PawnHealthComponent`)))))

(fn `Init Health Bar`
  (bind _asenemy_health_bar (cast `/Game/UnrealGameBP/Widget/EnemyHealthBar` (`WidgetComponent.GetWidget` (`self.HealthBar`))))
  (`/Game/UnrealGameBP/Widget/EnemyHealthBar.SetActor` _asenemy_health_bar self))

(fn `UserConstructionScript`)